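; BP_SpawnerBlocks decides which column and row cells of a grid are valid block positions; the file contains no spawning logic.
; IsValidBlockPosition switches between three pattern functions: both indices odd, checkerboard, or a single test cell.
; The switch is hard-coded to the test pattern, so only that one cell currently passes.
; The event graph and construction script are empty.
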(event EventBeginPlay)

(event Collision|EventActorBeginOverlap
  (params (OtherActor :type Actor%20Object%20Reference)))

(event EventTick
  (params (DeltaSeconds :type Float%20%28single-precision%29)))

(fn ConstructionScript)

(fn OddOddBlockPosition
  (params (Column :type Integer) (Row :type Integer))
  (return (and (!= (Math|Integer|%(Integer) Column 2) 0) (!= (Math|Integer|%(Integer) Row 2) 0))))

(fn IsValidBlockPosition
  (params (Column :type Integer) (Row :type Integer))
  (switch int 2
    (:0
      (bind _isvalid (CallFunction|OddOddBlockPosition Column Row))
      (LocalVariables|SetIsValid _isvalid))
    (:1
      (bind _isvalid_2 (CallFunction|ChessBlocksPosition Column Row))
      (LocalVariables|SetIsValid _isvalid_2))
    (:2
      (bind _isvalid_3 (CallFunction|TestBlockPosition Column Row))
      (LocalVariables|SetIsValid _isvalid_3)))
  (return (LocalVariables|GetIsValid)))

(fn ChessBlocksPosition
  (params (Column :type Integer) (Row :type Integer))
  (return (== (Math|Integer|%(Integer) (+ Column Row) 2) 0)))

(fn TestBlockPosition
  (params (Column :type Integer) (Row :type Integer))
  (return (and (== Column 3) (== Row 3))))